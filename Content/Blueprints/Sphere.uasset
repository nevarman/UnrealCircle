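; Sphere is a projectile-driven ball Blueprint that reacts to what it hits by checking the first tag on the other component.
; Hitting a "Player" component scales the ProjectileMovement velocity by SpeedUp, re-applied in local space, and calls OnUpdateScore.
; Hitting a "Finish" component zeroes the velocity and calls OnGameEnd, ending the round.
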(event OnComponentHit(Sphere)
  (params (OtherActor :type Actor%20Object%20Reference) (OtherComp :type Primitive%20Component%20Object%20Reference) (NormalImpulse :type Vector :default "0, 0, 0") (Hit :type Hit%20Result%20Structure%20%28by%20ref%29))
  (bind _componenttags (Variables|/Script/Engine.ActorComponent|GetComponentTags OtherComp))
  (bind _projectilemovement (Variables|Default|GetProjectileMovement))
  (bind _item (Utilities|Array|Get(acopy) _componenttags))
  (if (Utilities|Name|Equal(Name) _item "Player")
    (Game|Components|ProjectileMovement|SetVelocityinLocalSpace _projectilemovement (* (Variables|/Script/Engine.MovementComponent|GetVelocity _projectilemovement) (Variables|Default|GetSpeedUp)))
    (Default|CallOnUpdateScore)
    (elif (Utilities|Name|Equal(Name) _item "Finish")
      (Game|Components|ProjectileMovement|SetVelocityinLocalSpace "0, 0, 0")
      (Default|CallOnGameEnd))))

(event EventBeginPlay)

(fn ConstructionScript)